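; BP_Scroll is a keyboard-driven scroll effect built from a 17x17 grid of instanced meshes and a cylinder.
; Gates toggled by Q, Z and C let Tick randomly flip instances, drift them along X and blow them along Y with wraparound, through cached location and rotation arrays.
; X drives the scroll: a delayed-loop macro shifts the grid in Z one row at a time while a Timeline moves the cylinder.
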(event Custom|StartRotating
  (bind _deltaangle (Variables|Default|GetDeltaAngle))
  (bind _currotation (Variables|Default|GetCurRotation))
  (bind (_x _y) (Math|Vector|BreakVector _deltaangle))
  ;[1 1 1] 按Q翻转
  (Variables|Default|SetbRotating true)
  (Utilities|FlowControl|Gate true) ; enters at Open
)

(event Custom|StopMoving
  (bind _curlocation (Variables|Default|GetCurLocation))
  ;[1 1 1] 按Z纵向平移
  (Variables|Default|SetbMoving false)
  (Utilities|FlowControl|Gate true) ; enters at Close
)

(event Custom|StartMoving
  (bind _curlocation (Variables|Default|GetCurLocation))
  ;[1 1 1] 按Z纵向平移
  (Variables|Default|SetbMoving true)
  (Utilities|FlowControl|Gate true) ; enters at Open
)

(event Custom|TurningOn
  (bind _curlocation (Variables|Default|GetCurLocation))
  (bind _cylinder (Variables|Default|GetCylinder))
  (bind _returnvalue (Transformation|GetRelativeTransform _cylinder))
  (bind (_location _rotation _scale) (Math|Transform|BreakTransform _returnvalue))
  (bind (_x _y _z) (Math|Vector|BreakVector _location))
  ;[1 1 1] 按X模仿卷轴移动
  (Variables|Default|SetbTurningOn/Off true)
  (Utilities|FlowControl|Gate true) ; enters at Open
)

(event Custom|TruningOff
  (bind _curlocation (Variables|Default|GetCurLocation))
  (bind _cylinder (Variables|Default|GetCylinder))
  (bind _returnvalue (Transformation|GetRelativeTransform _cylinder))
  (bind (_location _rotation _scale) (Math|Transform|BreakTransform _returnvalue))
  (bind (_x _y _z) (Math|Vector|BreakVector _location))
  ;[1 1 1] 按X模仿卷轴移动
  (Variables|Default|SetbTurningOn/Off false)
  (Utilities|FlowControl|Gate true) ; enters at Close
)

(event Custom|BlowingAway
  (bind _curlocation (Variables|Default|GetCurLocation))
  ;[1 1 1] 按C结束
  (Utilities|FlowControl|Gate true) ; enters at Open
)

(event Custom|Over
  (bind _curlocation (Variables|Default|GetCurLocation))
  (bind _curlocation_2 (Variables|Default|GetCurLocation))
  (bind _deltaangle (Variables|Default|GetDeltaAngle))
  (bind _currotation (Variables|Default|GetCurRotation))
  (bind _curlocation_3 (Variables|Default|GetCurLocation))
  (bind _cylinder (Variables|Default|GetCylinder))
  (bind _returnvalue (Transformation|GetRelativeTransform _cylinder))
  (bind (_x _y) (Math|Vector|BreakVector _deltaangle))
  (bind (_location _rotation _scale) (Math|Transform|BreakTransform _returnvalue))
  (bind (_x_2 _y_2 _z) (Math|Vector|BreakVector _location))
  ;[1 1 1] 按C结束
  (Variables|Default|SetbOver true)
  (Utilities|FlowControl|Sequence
    (:then_0
      ;[1 1 1] 按Q翻转
      (Utilities|FlowControl|Gate true) ; enters at Close
    )
    (:then_1
      ;[1 1 1] 按Z纵向平移
      (Utilities|FlowControl|Gate true) ; enters at Close
    )
    (:then_2
      (Utilities|FlowControl|Gate true) ; enters at Close
    )
    (:then_3
      ;[1 1 1] 按X模仿卷轴移动
      (Utilities|FlowControl|Gate true) ; enters at Close
    )))

(event Custom|StopRotating
  (bind _deltaangle (Variables|Default|GetDeltaAngle))
  (bind _currotation (Variables|Default|GetCurRotation))
  (bind (_x _y) (Math|Vector|BreakVector _deltaangle))
  ;[1 1 1] 按Q翻转
  (for (_array_element _array_index) (Variables|Default|GetCurLocation)
    (Components|InstancedStaticMesh|UpdateInstanceTransform (Variables|Default|GetRow1) _array_index (Math|Transform|MakeTransform _array_element "0, 0, 0" "1,1,1") false true false)
    (Variables|Default|SetbRotating false)
    (Utilities|FlowControl|Gate true) ; enters at Close
  ))

(event EventBeginPlay
  (bind _locationarray (Variables|Default|GetLocationArray))
  (Input|EnableInput (Game|GetPlayerController 0))
  (Variables|Default|SetCurLocation _locationarray)
  (for (_ _array_index) _locationarray
    (Utilities|Array|Insert :TargetArray (Variables|Default|GetCurRotation) :Index _array_index)
    (Input|EnableInput (Game|GetPlayerController 0))))

(event Collision|EventActorBeginOverlap
  (params (OtherActor :type Actor%20Object%20Reference)))

(event EventTick
  (params (DeltaSeconds :type Float%20%28single-precision%29))
  (bind _curlocation (Variables|Default|GetCurLocation))
  (bind _deltaangle (Variables|Default|GetDeltaAngle))
  (bind _currotation (Variables|Default|GetCurRotation))
  (bind _curlocation_2 (Variables|Default|GetCurLocation))
  (bind (_x _y) (Math|Vector|BreakVector _deltaangle))
  ;[1 1 1] 按Q翻转
  (Variables|Default|SetDeltaTime DeltaSeconds)
  (Utilities|FlowControl|Sequence
    (:then_0
      ;[1 1 1] 按Z纵向平移
      (Utilities|FlowControl|Gate true
        (:Exit
          (for (_array_element _array_index) _curlocation_2
            (if (>= (Math|Random|RandomFloat) 0.4)
              (if (>= (.X (Math|Vector|BreakVector (+ _array_element (Math|Vector|MakeVector (* (Variables|Default|GetMovingSpeed) (Variables|Default|GetDeltaTime)) 0.0 0.0)))) -25.0)
                (Utilities|Array|SetArrayElem _curlocation_2 _array_index (Math|Vector|MakeVector -1.92e+03 (.Y (Math|Vector|BreakVector (+ _array_element (Math|Vector|MakeVector (* (Variables|Default|GetMovingSpeed) (Variables|Default|GetDeltaTime)) 0.0 0.0)))) (.Z (Math|Vector|BreakVector (+ _array_element (Math|Vector|MakeVector (* (Variables|Default|GetMovingSpeed) (Variables|Default|GetDeltaTime)) 0.0 0.0))))))
                (else
                  (Utilities|Array|SetArrayElem _curlocation_2 _array_index (+ _array_element (Math|Vector|MakeVector (* (Variables|Default|GetMovingSpeed) (Variables|Default|GetDeltaTime)) 0.0 0.0))))))))))
    (:then_1
      (Utilities|FlowControl|Gate true
        (:Exit
          (for (_array_element_2 _array_index_2) (Variables|Default|GetCurLocation)
            (if (>= (Math|Random|RandomFloat) 0.5)
              (Utilities|Array|SetArrayElem _currotation _array_index_2 (Math|Rotator|MakeRotator (+ _x (.Roll (Math|Rotator|BreakRotator (Utilities|Array|Get(acopy) _currotation _array_index_2)))) (+ _y (.Pitch (Math|Rotator|BreakRotator (Utilities|Array|Get(acopy) _currotation _array_index_2)))) -45.0))
              (Components|InstancedStaticMesh|UpdateInstanceTransform (Variables|Default|GetRow1) _array_index_2 (Math|Transform|MakeTransform _array_element_2 (Math|Rotator|MakeRotator (+ _x (.Roll (Math|Rotator|BreakRotator (Utilities|Array|Get(acopy) _currotation _array_index_2)))) (+ _y (.Pitch (Math|Rotator|BreakRotator (Utilities|Array|Get(acopy) _currotation _array_index_2)))) -45.0) "1,1,1") false true false))))))
    (:then_2
      ;[1 1 1] 按C结束
      (Utilities|FlowControl|Gate true
        (:Exit
          (for (_array_element_3 _array_index_3) _curlocation
            (if (>= (.Y (Math|Vector|BreakVector (+ _array_element_3 (Math|Vector|MakeVector 0.0 (* (Variables|Default|GetBlowingSpeed) (Variables|Default|GetDeltaTime)) 0.0)))) 1.86e+03)
              (Utilities|Array|SetArrayElem _curlocation _array_index_3 (Utilities|Array|Get(acopy) (Variables|Default|GetLocationArray) _array_index_3))
              (else
                (Utilities|Array|SetArrayElem _curlocation _array_index_3 (+ _array_element_3 (Math|Vector|MakeVector 0.0 (* (Variables|Default|GetBlowingSpeed) (Variables|Default|GetDeltaTime)) 0.0)))))))))))

(event Input|KeyboardEvents|X
  (params (Key :type Key%20Structure :default "None"))
  ;[1 1 1] 控制栏
  ;;[1 1 1] 卷轴移动
  (:Pressed
    (Development|PrintString "X pressed")
    (if (Variables|Default|GetbTurningOn/Off)
      (CallFunction|TruningOff)
      (else
        (CallFunction|Turningon)))))

(event Input|KeyboardEvents|Q
  (params (Key :type Key%20Structure :default "None"))
  ;[1 1 1] 控制栏
  ;;[1 1 1] 翻转
  (:Pressed
    (Development|PrintString "Q pressed")
    (if (Variables|Default|GetbRotating)
      (CallFunction|StopRotating)
      (else
        (CallFunction|StartRotating)))))

(event Input|KeyboardEvents|C
  (params (Key :type Key%20Structure :default "None"))
  ;[1 1 1] 控制栏
  ;;[1 1 1] 流程结束
  (:Pressed
    (Development|PrintString "C pressed")
    (if (not (Variables|Default|GetbOver))
      (CallFunction|BlowingAway))))

(event Input|KeyboardEvents|Z
  (params (Key :type Key%20Structure :default "None"))
  ;[1 1 1] 控制栏
  ;;[1 1 1] 纵向平移
  (:Pressed
    (Development|PrintString "Z pressed")
    (if (Variables|Default|GetbMoving)
      (CallFunction|StopMoving)
      (else
        (CallFunction|StartMoving)))))

(event Input|KeyboardEvents|X
  (params (Key :type Key%20Structure :default "None"))
  (bind _curlocation (Variables|Default|GetCurLocation))
  (bind _cylinder (Variables|Default|GetCylinder))
  (bind _returnvalue (Transformation|GetRelativeTransform _cylinder))
  (bind (_location _rotation _scale) (Math|Transform|BreakTransform _returnvalue))
  (bind (_x _y _z) (Math|Vector|BreakVector _location))
  ;[1 1 1] 按X模仿卷轴移动
  (:Pressed
    (Utilities|FlowControl|Gate true
      (:Exit
        (Utilities|FlowControl|Sequence
          (:then_0
            ;;[1 1 1] 改Duration可以修改前展开时间
            (bind _index (Utilities|ForLoopwithDelay 0 16 0.7)
              (:Loop%20Body
                (for _index_2 (range 0 16)
                  (Utilities|Array|SetArrayElem _curlocation (+ (* _index 17) _index_2) (Math|Vector|MakeVector (.X (Math|Vector|BreakVector (Utilities|Array|Get(acopy) _curlocation (+ (* _index 17) _index_2)))) (.Y (Math|Vector|BreakVector (Utilities|Array|Get(acopy) _curlocation (+ (* _index 17) _index_2)))) 6e+03))
                  (Components|InstancedStaticMesh|UpdateInstanceTransform (Variables|Default|GetRow1) (+ (* _index 17) _index_2) (Math|Transform|MakeTransform (Utilities|Array|Get(acopy) _curlocation (+ (* _index 17) _index_2)) (Utilities|Array|Get(acopy) (Variables|Default|GetCurRotation) (+ (* _index 17) _index_2)) "1,1,1") false true false)))))
          (:then_1
            ;[1 1 1] 圆柱体滚动
            (bind _newtrack_0 (Timeline|Timeline_0 Play)
              (:Update
                (Transformation|SetRelativeTransform _cylinder (Math|Transform|MakeTransform (Math|Vector|MakeVector _x _newtrack_0 _z) _rotation _scale) false false)))))))))

(fn ConstructionScript
  (for _index (range 1 17)
    (for _index_2 (range 1 17)
      (Components|InstancedStaticMesh|AddInstance (Variables|Default|GetRow1) (Math|Transform|MakeTransform (Variables|Default|GetLocation) "0, 0, 0" "0.700000,0.700000,0.700000"))
      (Utilities|Array|Add (Variables|Default|GetLocationArray) (Variables|Default|GetLocation))
      (Variables|Default|SetLocation (+ (Variables|Default|GetLocation) (Variables|Default|GetDeltaLocationX))))
    (bind _output_get (Variables|Default|SetStartLocation (+ (Variables|Default|GetStartLocation) (Variables|Default|GetDeltaLocationY))))
    (Variables|Default|SetLocation _output_get)))