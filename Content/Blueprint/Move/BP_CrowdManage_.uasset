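; Crowd manager actor that spawns a field of BP_SingleOne actors from a data table and animates a ripple wave through them.
; ReadData loads initial positions from InitTable, and AddActors spawns one scaled actor per row into the Crowd array.
; While BBegin is set, Tick advances a timer and runs Updowm, raising members inside an expanding distance band around a fixed center and resetting the rest to ground height.
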(event EventBeginPlay
  (Variables|Default|SetCurTime 0.0)
  (Variables|Default|SetBeiMoveTime 0.0)
  (Variables|Default|SetJingMoveTime 0.0)
  (Variables|Default|SetBackMoveTime 0.0)
  (Variables|Default|SetSLigntTime 0.0)
  (Variables|Default|SetSMoveLight_2 0.0)
  (Variables|Default|SetRandomLightTime 0.0)
  (Variables|Default|SetDarkTime 0.0)
  (Variables|Default|SetLinetime 0.0)
  (Variables|Default|SetLineDarkTime 0.0)
  (Variables|Default|SetRandomTime 0.0))

(event Collision|EventActorBeginOverlap
  (params (OtherActor :type Actor%20Object%20Reference)))

(event EventTick
  (params (DeltaSeconds :type Float%20%28single-precision%29))
  (Variables|Default|SetDeltaTime DeltaSeconds)
  (if (Variables|Default|GetB_Begin)
    (Variables|Default|SetCurTime (+ (Variables|Default|GetCurTime) (Variables|Default|GetDeltaTime)))
    (CallFunction|Updowm)))

(fn ConstructionScript)

(fn ReadData
  (bind _inittable (Variables|Default|GetinitTable))
  (bind _outrownames (DataTable|GetDataTableRowNames _inittable))
  ;[1 1 1] 初始位置数据
  (for _array_element _outrownames
    (bind _returnvalue (Utilities|GetDataTableRow _inittable _array_element)
      (:then
        (Utilities|Array|Add (Variables|Default|GetInitMoveData) _returnvalue))
      (:RowNotFound
        (Development|PrintString "读取数据表失败")))))

(fn AddActors
  (for _array_element (Variables|Default|GetInitMoveData)
    (bind _returnvalue (Game|SpawnActorfromClass "/Game/Blueprint/Move/BP_SingleOne.BP_SingleOne_C" (Math|Transform|MakeTransform (Math|Vector|MakeVector (.InstanceX (Utilities|Struct|BreakS_InitialData _array_element)) (.InstanceY (Utilities|Struct|BreakS_InitialData _array_element)) 0.0) "0, 0, 0" "5.000000,5.000000,5.000000") "Undefined" 0 0))
    (Utilities|Array|Add (Variables|Default|GetCrowd) _returnvalue)))

(fn Updowm
  (bind _curtime (Variables|Default|GetCurTime))
  (for (_array_element _array_index) (Variables|Default|GetCrowd)
    (if (Math|Float|InRange(Float) (Math|Float|Absolute(Float) (Math|Vector|Distance(Vector) (Math|Vector|MakeVector (.InstanceX (Utilities|Struct|BreakS_InitialData (Utilities|Array|Get(acopy) (Variables|Default|GetInitMoveData) _array_index))) (.InstanceY (Utilities|Struct|BreakS_InitialData (Utilities|Array|Get(acopy) (Variables|Default|GetInitMoveData) _array_index))) 0.0) "900.000000,1400.000000, 0")) (* (- _curtime 1.0) 5e+02) (* _curtime 5e+02))
      (Transformation|SetWorldLocation (Variables|/Game/Blueprint/Move/BP_SingleOne.BP_SingleOne_C|GetSingleOne _array_element) (Math|Vector|MakeVector (.InstanceX (Utilities|Struct|BreakS_InitialData (Utilities|Array|Get(acopy) (Variables|Default|GetInitMoveData) _array_index))) (.InstanceY (Utilities|Struct|BreakS_InitialData (Utilities|Array|Get(acopy) (Variables|Default|GetInitMoveData) _array_index))) 1e+02) false false)
      (else
        (Transformation|SetWorldLocation (Variables|/Game/Blueprint/Move/BP_SingleOne.BP_SingleOne_C|GetSingleOne _array_element) (Math|Vector|MakeVector (.InstanceX (Utilities|Struct|BreakS_InitialData (Utilities|Array|Get(acopy) (Variables|Default|GetInitMoveData) _array_index))) (.InstanceY (Utilities|Struct|BreakS_InitialData (Utilities|Array|Get(acopy) (Variables|Default|GetInitMoveData) _array_index))) 0.0) false false)))))