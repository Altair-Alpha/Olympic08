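; Crowd actor that animates instanced meshes placed from data table positions, raising them in successive groups like a wave.
; The construction script reads the initial and north position tables, spawns the instances and creates dynamic materials.
; Tick drives Move1, which lifts a time-based index window and lowers the rest on a repeating cycle; its color switch is noted as failing.
; Move2, an interpolation toward the north positions, is never called, and Move3 is empty.
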(event Custom|beginPlay
  (CallFunction|Move1))

(event EventBeginPlay
  (Variables|Default|SetCurTime 0.0))

(event Collision|EventActorBeginOverlap
  (params (OtherActor :type Actor%20Object%20Reference)))

(event EventTick
  (params (DeltaSeconds :type Float%20%28single-precision%29))
  ;[1 1 1] 初始化每帧时间和当前时间
  (bind _output_get (Variables|Default|SetDeltaTime DeltaSeconds))
  (Variables|Default|SetCurTime (+ _output_get (Variables|Default|GetCurTime)))
  (CallFunction|Move1))

(fn ConstructionScript
  (CallFunction|ReadData)
  (CallFunction|AddInstance))

(fn ReadData
  (bind _initmovetable (Variables|Default|GetInitMoveTable))
  (bind _northmovetable (Variables|Default|GetNorthMoveTable))
  (bind _outrownames (DataTable|GetDataTableRowNames _initmovetable))
  (for _array_element _outrownames
    (bind _returnvalue (Utilities|GetDataTableRow _initmovetable _array_element)
      (:then
        (Utilities|Array|Add (Variables|Default|GetInitMoveData) _returnvalue))
      (:RowNotFound
        (Development|PrintString "读取数据表失败"))))
  (bind _outrownames_2 (DataTable|GetDataTableRowNames _northmovetable))
  (for _array_element_2 _outrownames_2
    (bind _returnvalue_2 (Utilities|GetDataTableRow _northmovetable _array_element_2)
      (:then
        (Utilities|Array|Add (Variables|Default|GetNorthMoveData) _returnvalue_2))
      (:RowNotFound
        (Development|PrintString "读取数据表失败")))))

(fn AddInstance
  (bind _crowd (Variables|Default|Getcrowd))
  (for _array_element (Variables|Default|GetInitMoveData)
    (bind _returnvalue (Class|InstancedStaticMeshComponent|AddInstanceWorldSpace (Variables|Default|Getcrowd) (Math|Transform|MakeTransform (Math|Vector|MakeVector (.InstanceX (Utilities|Struct|BreakS_InitialData _array_element)) (.InstanceY (Utilities|Struct|BreakS_InitialData _array_element)) 8e+02) "0, 0, 0" "2.400000,2.400000,2.400000")))
    (bind _returnvalue_2 (Rendering|Material|CreateDynamicMaterialInstance _crowd _returnvalue (Utilities|Array|Get(acopy) (Rendering|Material|GetMaterials _crowd) 3) "None" :!class /Script/Engine.PrimitiveComponent))
    (Variables|Default|SetIDM _returnvalue_2)
    (Rendering|Material|SetMaterial (Variables|Default|Getcrowd) _returnvalue _returnvalue_2)))

(fn Move1
  (bind _crowd (Variables|Default|Getcrowd))
  (bind _crowd_2 (Variables|Default|Getcrowd))
  (bind _crowd_3 (Variables|Default|Getcrowd))
  (bind _returnvalue (Transformation|GetWorldScale _crowd))
  (if (< (Variables|Default|GetCurTime) 3e+01)
    (for (_array_element _array_index) (Variables|Default|GetInitMoveData)
      (if (Math|Float|InRange(Float) (Math|Conversions|ToFloat(Integer) _array_index) (* (Variables|Default|GetCurTime) 21.0) (* (+ (Variables|Default|GetCurTime) 1.0) 21.0))
        (Components|InstancedStaticMesh|UpdateInstanceTransform _crowd_3 _array_index (Math|Transform|MakeTransform (Math|Vector|MakeVector (.InstanceX (Utilities|Struct|BreakS_InitialData _array_element)) (.InstanceY (Utilities|Struct|BreakS_InitialData _array_element)) 8e+02) "0, 0, 0" _returnvalue) false false false)
        (else
          (Components|InstancedStaticMesh|UpdateInstanceTransform _crowd_3 _array_index (Math|Transform|MakeTransform (Math|Vector|MakeVector (.InstanceX (Utilities|Struct|BreakS_InitialData _array_element)) (.InstanceY (Utilities|Struct|BreakS_InitialData _array_element)) 5e+02) "0, 0, 0" _returnvalue) false false false)
          ;[1 1 1] 切换颜色-失败
          (Rendering|Material|SetVectorParameterValue (Variables|Default|GetIDM) "BaseColor" (Utilities|Struct|MakeLinearColor 0.0 0.0 0.0 1.0) :!class /Script/Engine.MaterialInstanceDynamic))))
    (Components|InstancedStaticMesh|UpdateInstanceTransform _crowd_2 0 (.OutInstanceTransform (Components|InstancedStaticMesh|GetInstanceTransform _crowd_2 0 false)) false true false)
    (else
      (Variables|Default|SetCurTime 0.0))))

(fn Move2
  (bind _crowd (Variables|Default|Getcrowd))
  (bind _crowd_2 (Variables|Default|GetCrowd))
  (bind (_outinstancetransform _returnvalue) (Components|InstancedStaticMesh|GetInstanceTransform _crowd 0 false))
  (if (<= (Variables|Default|GetCurTime) (Variables|Default|GetTotalTime))
    (bind (_array_element _array_index) (Utilities|Array|ForEachLoopwithBreak (Variables|Default|GetInitMoveData))
      (:LoopBody
        (Components|InstancedStaticMesh|UpdateInstanceTransform _crowd_2 _array_index (Math|Transform|MakeTransform (+ (Math|Vector|MakeVector (.InstanceX (Utilities|Struct|BreakS_InitialData _array_element)) (.InstanceY (Utilities|Struct|BreakS_InitialData _array_element)) 0.0) (* (- (Math|Vector|MakeVector (.InstanceX (Utilities|Struct|BreakS_NorthMove (Utilities|Array|Get(acopy) (Variables|Default|GetNorthMoveData) _array_index))) (.InstanceY (Utilities|Struct|BreakS_NorthMove (Utilities|Array|Get(acopy) (Variables|Default|GetNorthMoveData) _array_index))) 0.0) (Math|Vector|MakeVector (.InstanceX (Utilities|Struct|BreakS_InitialData _array_element)) (.InstanceY (Utilities|Struct|BreakS_InitialData _array_element)) 0.0)) (/ (Variables|Default|GetCurTime) (Variables|Default|GetTotalTime)))) "0, 0, 0" (Transformation|GetWorldScale _crowd_2)) false false false))
      (:Completed
        (Components|InstancedStaticMesh|UpdateInstanceTransform _crowd 0 _outinstancetransform _returnvalue true false)))))

(fn Move3)

(fn Time)