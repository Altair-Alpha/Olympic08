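; Crowd manager that spawns BP_CrowdActor instances from data-table positions and switches selected ones bright or dark, apparently for crowd-formed characters.
; ReadData loads initial and "北" (North) layouts, and AddInstance spawns half-scale actors from the initial one; neither is called here.
; ChangeDigit drives TurnBright/TurnDark by index arrays; an Enter-key test feeds it odd indices.
; North data goes unused, ChangeCharBei/ChangeCharJing are empty, and Tick only accumulates time.
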(event EventBeginPlay
  (Variables|Default|SetCurTime 0.0))

(event Collision|EventActorBeginOverlap
  (params (OtherActor :type Actor%20Object%20Reference)))

(event EventTick
  (params (DeltaSeconds :type Float%20%28single-precision%29))
  ;[1 1 1] 初始化每帧时间和当前时间
  (bind _output_get (Variables|Default|SetDeltaTime DeltaSeconds))
  (Variables|Default|SetCurTime (+ _output_get (Variables|Default|GetCurTime))))

(event Input|KeyboardEvents|Enter
  (params (Key :type Key%20Structure :default "None"))
  (:Pressed
    (for _index (range 0 299)
      (Utilities|Array|Add (Variables|Default|GetTestArrBright) (+ (* _index 2) 1))
      (CallFunction|ChangeDigit (Variables|Default|GetTestArrBright) (Variables|Default|GetTestArrDark)))))

(fn ConstructionScript)

(fn ReadData
  (bind _initmovetable (Variables|Default|GetInitMoveTable))
  (bind _northmovetable (Variables|Default|GetNorthMoveTable))
  (bind _outrownames (DataTable|GetDataTableRowNames _initmovetable))
  ;[1 1 1] 初始位置数据
  (for _array_element _outrownames
    (bind _returnvalue (Utilities|GetDataTableRow _initmovetable _array_element)
      (:then
        (Utilities|Array|Add (Variables|Default|GetInitMoveData) _returnvalue))
      (:RowNotFound
        (Development|PrintString "读取数据表失败"))))
  ;[1 1 1] 北字数据
  (bind _outrownames_2 (DataTable|GetDataTableRowNames _northmovetable))
  (for _array_element_2 _outrownames_2
    (bind _returnvalue_2 (Utilities|GetDataTableRow _northmovetable _array_element_2)
      (:then
        (Utilities|Array|Add (Variables|Default|GetNorthMoveData) _returnvalue_2))
      (:RowNotFound
        (Development|PrintString "读取数据表失败")))))

(fn AddInstance
  (for _array_element (Variables|Default|GetInitMoveData)
    (bind _returnvalue (Game|SpawnActorfromClass "/Game/Blueprint/Move/BP_CrowdActor.BP_CrowdActor_C" (Math|Transform|MakeTransform (Math|Vector|MakeVector (.InstanceX (Utilities|Struct|BreakS_InitialData _array_element)) (.InstanceY (Utilities|Struct|BreakS_InitialData _array_element)) 0.0) "0, 0, 0" "0.500000,0.500000,0.500000") "Undefined" 0 0))
    (Utilities|Array|Add (Variables|Default|GetCrowd) _returnvalue)))

(fn ChangeDigit
  (params (BrightPosArr :type Array%20of%20Integers) (DarkPosArr :type Array%20of%20Integers))
  (Utilities|FlowControl|Sequence
    (:then_0
      (for _array_element BrightPosArr
        (Default|TurnBright (Utilities|Array|Get(acopy) (Variables|Default|GetCrowd) _array_element))))
    (:then_1
      (for _array_element_2 DarkPosArr
        (Default|TurnDark (Utilities|Array|Get(acopy) (Variables|Default|GetCrowd) _array_element_2))))))

(fn ChangeCharBei)

(fn ChangeCharJing)