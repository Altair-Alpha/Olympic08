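; BP_CrowdActor is a crowd actor whose cube switches between bright and dark looks, either instantly or as a fade.
; TurnBright and TurnDark assign the MBright or MDark material directly.
; FadeBright and FadeDark play timelines that drive the EmisColor parameter on a dynamic material instance and apply it to the cube.
; The construction script creates that instance from the cube's current material.
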(event Custom|FadeBright
  (bind _dmi (Variables|Default|GetDMI))
  (bind _emiscolor (Timeline|TurnBright_Timeline PlayFromStart)
    (:Update
      (Rendering|Material|SetVectorParameterValue _dmi "EmisColor" _emiscolor :!class /Script/Engine.MaterialInstanceDynamic)
      (Rendering|Material|SetMaterial (Variables|Default|GetCube) 0 _dmi))))

(event Custom|FadeDark
  (bind _dmi (Variables|Default|GetDMI))
  (bind _emiscolor (Timeline|TurnDark_Timeline PlayFromStart)
    (:Update
      (Rendering|Material|SetVectorParameterValue _dmi "EmisColor" _emiscolor :!class /Script/Engine.MaterialInstanceDynamic)
      (Rendering|Material|SetMaterial (Variables|Default|GetCube) 0 _dmi))))

(event Custom|TurnBright
  (Rendering|Material|SetMaterial (Variables|Default|GetCube) 0 (Variables|Default|GetM_Bright)))

(event Custom|TurnDark
  (Rendering|Material|SetMaterial (Variables|Default|GetCube) 0 (Variables|Default|GetM_Dark)))

(fn ConstructionScript
  (bind _returnvalue (Rendering|Material|CreateDynamicMaterialInstance (Rendering|Material|GetMaterial (Variables|Default|GetCube) 0) "None" :!class /Script/Engine.KismetMaterialLibrary))
  (Variables|Default|SetDMI _returnvalue))