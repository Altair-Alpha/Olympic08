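; Crowd manager Blueprint that spawns a grid or layout of BP_SingleOne actors from a data table and animates their height over time.
; ReadData loads rows into InitData, and AddActor spawns one actor per X/Y entry into Crowd.
; While Begin is set, Tick accumulates time and SMove lifts 20 more members per second by index.
; Members not yet lifted stay at ground level and receive TurnBright every frame.
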(event Custom|BeginPlay)

(event EventBeginPlay
  (Variables|Default|SetcurTime 0.0)
  (Variables|Default|SetTotalTime 5e+01)
  (Development|PrintString (Utilities|String|ToString(Integer) (Utilities|Array|Length (Variables|Default|GetIDM_color)))))

(event Collision|EventActorBeginOverlap
  (params (OtherActor :type Actor%20Object%20Reference)))

(event EventTick
  (params (DeltaSeconds :type Float%20%28single-precision%29))
  (bind _output_get (Variables|Default|SetDeltaTime DeltaSeconds))
  (if (Variables|Default|Getbegin)
    (Variables|Default|SetcurTime (+ _output_get (Variables|Default|GetcurTime)))
    (CallFunction|SMove)))

(fn ConstructionScript)

(fn ReadData
  (bind _initdatatable (Variables|Default|GetInitDataTable))
  (bind _outrownames (DataTable|GetDataTableRowNames _initdatatable))
  (for _array_element _outrownames
    (bind _returnvalue (Utilities|GetDataTableRow _initdatatable _array_element)
      (:then
        (Utilities|Array|Add (Variables|Default|GetInitData) _returnvalue))
      (:RowNotFound
        (Development|PrintString "数据读取失败")))))

(fn AddActor
  (for _array_element (Variables|Default|GetInitData)
    (bind _returnvalue (Game|SpawnActorfromClass "/Game/Blueprint/Move/BP_SingleOne.BP_SingleOne_C" (Math|Transform|MakeTransform (Math|Vector|MakeVector (.InstanceX (Utilities|Struct|BreakS_InitialData _array_element)) (.InstanceY (Utilities|Struct|BreakS_InitialData _array_element)) 0.0) "0, 0, 0" "1,1,1") "Undefined" 0 0))
    (bind _returnvalue_2 (Utilities|Array|Add (Variables|Default|GetCrowd) _returnvalue))))

(fn SMove
  (for (_array_element _array_index) (Variables|Default|GetCrowd)
    (if (< _array_index (* (Math|Float|Truncate (Variables|Default|GetcurTime)) 20))
      (Transformation|SetWorldLocation (Variables|/Game/Blueprint/Move/BP_SingleOne.BP_SingleOne_C|GetSingleOne _array_element) (Math|Vector|MakeVector (.InstanceX (Utilities|Struct|BreakS_InitialData (Utilities|Array|Get(acopy) (Variables|Default|GetInitData) _array_index))) (.InstanceY (Utilities|Struct|BreakS_InitialData (Utilities|Array|Get(acopy) (Variables|Default|GetInitData) _array_index))) 2e+02) false false)
      (else
        (Transformation|SetWorldLocation (Variables|/Game/Blueprint/Move/BP_SingleOne.BP_SingleOne_C|GetSingleOne _array_element) (Math|Vector|MakeVector (.InstanceX (Utilities|Struct|BreakS_InitialData (Utilities|Array|Get(acopy) (Variables|Default|GetInitData) _array_index))) (.InstanceY (Utilities|Struct|BreakS_InitialData (Utilities|Array|Get(acopy) (Variables|Default|GetInitData) _array_index))) 0.0) false false)
        (Default|TurnBright _array_element)))))