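; Firework show manager that times Niagara effects for an Olympic-themed performance at hard-coded world positions.
; Three top-level events use delays to stage opening small and large fireworks, the Olympic rings, and a flower bloom with petal spread followed by a blue map effect.
; Small fireworks fire in a staggered ring, large ones burst together, and map effects appear at random intervals.
; Completion and map-start calls signal stage progress.
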(event Custom|FireworkBegin_L
  ;[1 1 1] 开场大烟花事件调度
  (Utilities|FlowControl|Delay 1.0)
  (Utilities|FlowControl|Sequence
    (:then_0
      (Niagara|SpawnSystematLocation (Variables|Default|GetFirework_L) "4440.000000,3590.000000,7540.000000"))
    (:then_1
      (Niagara|SpawnSystematLocation (Variables|Default|GetFirework_L) "5330.000000,-50.000000,7540.000000"))
    (:then_2
      (Niagara|SpawnSystematLocation (Variables|Default|GetFirework_L) "4520.000000,-3200.000000,7540.000000"))
    (:then_3
      (Niagara|SpawnSystematLocation (Variables|Default|GetFirework_L) "1500.000000,-5900.000000,7540.000000"))
    (:then_4
      (Niagara|SpawnSystematLocation (Variables|Default|GetFirework_L) "-2160.000000,-5930.000000,7540.000000"))
    (:then_5
      (Niagara|SpawnSystematLocation (Variables|Default|GetFirework_L) "-4720.000000,-2690.000000,7540.000000"))
    (:then_6
      (Niagara|SpawnSystematLocation (Variables|Default|GetFirework_L) "-5200.000000,1150.000000,7540.000000"))
    (:then_7
      (Niagara|SpawnSystematLocation (Variables|Default|GetFirework_L) "-3130.000000,5190.000000,7540.000000"))
    (:then_8
      (Niagara|SpawnSystematLocation (Variables|Default|GetFirework_L) "1030.000000,5610.000000,7540.000000"))))

(event Custom|FireworkBegin_S
  ;[1 1 1] 开场小烟花事件调度
  (Utilities|FlowControl|Delay 0.5)
  (Niagara|SpawnSystematLocation (Variables|Default|GetFirework_S) "1520.000000,4890.000000,500.000000")
  (Utilities|FlowControl|Delay 0.5)
  (Niagara|SpawnSystematLocation (Variables|Default|GetFirework_S) "0.000000,5490.000000,500.000000")
  (Utilities|FlowControl|Delay 0.5)
  (Niagara|SpawnSystematLocation (Variables|Default|GetFirework_S) "-1520.000000,4890.000000,500.000000")
  (Utilities|FlowControl|Delay 0.5)
  (Niagara|SpawnSystematLocation (Variables|Default|GetFirework_S) "-2980.000000,4250.000000,500.000000")
  (Utilities|FlowControl|Delay 0.5)
  (Niagara|SpawnSystematLocation (Variables|Default|GetFirework_S) "-3740.000000,1800.000000,500.000000")
  (Utilities|FlowControl|Delay 0.5)
  (Niagara|SpawnSystematLocation (Variables|Default|GetFirework_S) "-3740.000000,280.000000,500.000000")
  (Utilities|FlowControl|Delay 0.5)
  (Niagara|SpawnSystematLocation (Variables|Default|GetFirework_S) "-3740.000000,-1070.000000,500.000000")
  (Utilities|FlowControl|Delay 0.5)
  (Niagara|SpawnSystematLocation (Variables|Default|GetFirework_S) "-2980.000000,-4250.000000,500.000000")
  (Utilities|FlowControl|Delay 0.5)
  (Niagara|SpawnSystematLocation (Variables|Default|GetFirework_S) "-1520.000000,-4890.000000,500.000000")
  (Utilities|FlowControl|Delay 0.5)
  (Niagara|SpawnSystematLocation (Variables|Default|GetFirework_S) "0.000000,-5490.000000,500.000000")
  (Utilities|FlowControl|Delay 0.5)
  (Niagara|SpawnSystematLocation (Variables|Default|GetFirework_S) "1520.000000,-4890.000000,500.000000")
  (Utilities|FlowControl|Delay 0.5)
  (Niagara|SpawnSystematLocation (Variables|Default|GetFirework_S) "2980.000000,-4250.000000,500.000000")
  (Utilities|FlowControl|Delay 0.5)
  (Niagara|SpawnSystematLocation (Variables|Default|GetFirework_S) "3740.000000,-1070.000000,500.000000")
  (Utilities|FlowControl|Delay 0.5)
  (Niagara|SpawnSystematLocation (Variables|Default|GetFirework_S) "3740.000000,280.000000,500.000000")
  (Utilities|FlowControl|Delay 0.5)
  (Niagara|SpawnSystematLocation (Variables|Default|GetFirework_S) "3740.000000,1800.000000,500.000000")
  (Utilities|FlowControl|Delay 0.5)
  (Niagara|SpawnSystematLocation (Variables|Default|GetFirework_S) "2980.000000,4250.000000,500.000000"))

(event Custom|FireworkBegin
  ;[1 1 1] Dispatcher1
  (Utilities|FlowControl|Delay 2.0)
  (CallFunction|FireworkBeginS)
  (Utilities|FlowControl|Delay 15.0)
  (CallFunction|FireworkBeginL)
  (Utilities|FlowControl|Delay 2e+01)
  (Default|CallFireworkBeginComplete))

(event Custom|OlympicCireclesEmerge
  ;[1 1 1] 五环事件调度
  (Niagara|SpawnSystematLocation (Variables|Default|GetOlympicCircles) "-800.000000, 0,2000.000000" "0,-90.000000,90.000000" "80.000000,80.000000,10.000000"))

(event Custom|FlowerBloom
  ;[1 1 1] 花朵特效事件调度
  (Niagara|SpawnSystematLocation (Variables|Default|GetFlower) "0.000000,350.000000,1800.000000" "0,-90.000000,0.000000" "120.000000,120.000000,120.000000"))

(event Custom|FlowerSpread
  ;[1 1 1] 花瓣散开事件调度
  (Niagara|SpawnSystematLocation (Variables|Default|GetPieceSpread) "0,350.000000,800.000000"))

(event Custom|BlueMap
  ;[1 1 1] 底图特效事件调度
  (Utilities|FlowControl|Delay (Math|Random|RandomFloatinRange 0.0 0.8))
  (Niagara|SpawnSystematLocation (Variables|Default|GetBlue) "-20.000000,1480.000000,710.000000")
  (Utilities|FlowControl|Delay (Math|Random|RandomFloatinRange 0.0 0.8))
  (Niagara|SpawnSystematLocation (Variables|Default|GetBlue) "280.000000,-2930.000000,710.000000")
  (Utilities|FlowControl|Delay (Math|Random|RandomFloatinRange 0.0 0.8))
  (Niagara|SpawnSystematLocation (Variables|Default|GetBlue) "950.000000,-2040.000000,710.000000")
  (Utilities|FlowControl|Delay (Math|Random|RandomFloatinRange 0.0 0.8))
  (Niagara|SpawnSystematLocation (Variables|Default|GetBlue) "-360.000000,-2780.000000,710.000000")
  (Utilities|FlowControl|Delay (Math|Random|RandomFloatinRange 0.0 0.8))
  (Niagara|SpawnSystematLocation (Variables|Default|GetBlue) "-810.000000,-1940.000000,710.000000")
  (Utilities|FlowControl|Delay (Math|Random|RandomFloatinRange 0.0 0.8))
  (Niagara|SpawnSystematLocation (Variables|Default|GetBlue) "-220.000000,1550.000000,710.000000")
  (Utilities|FlowControl|Delay (Math|Random|RandomFloatinRange 0.0 0.8))
  (Niagara|SpawnSystematLocation (Variables|Default|GetBlue) "380.000000,2320.000000,710.000000")
  (Utilities|FlowControl|Delay (Math|Random|RandomFloatinRange 0.0 0.8))
  (Niagara|SpawnSystematLocation (Variables|Default|GetBlue) "1030.000000,1630.000000,710.000000")
  (Utilities|FlowControl|Delay (Math|Random|RandomFloatinRange 0.0 0.8))
  (Niagara|SpawnSystematLocation (Variables|Default|GetBlue) "-680.000000,1970.000000,710.000000")
  (Utilities|FlowControl|Delay (Math|Random|RandomFloatinRange 0.0 0.8))
  (Niagara|SpawnSystematLocation (Variables|Default|GetBlue) "-170.000000,2530.000000,710.000000"))

(event Custom|Performance1
  ;[1 1 1] Dispatcher2
  (CallFunction|OlympicCireclesEmerge)
  (Utilities|FlowControl|Delay 55.0)
  (Default|CallOlympicComplete))

(event Custom|Performance2
  ;[1 1 1] Dispatcher3
  (Utilities|FlowControl|Sequence
    (:then_0
      (CallFunction|FlowerBloom))
    (:then_1
      (CallFunction|FlowerSpread)
      (Utilities|FlowControl|Delay 48.0)
      (CallFunction|BlueMap)
      (Default|CallMapStart))))

(fn ConstructionScript)