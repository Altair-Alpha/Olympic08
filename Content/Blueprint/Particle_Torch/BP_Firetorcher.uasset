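; BP_Firetorcher is a torch-bearer actor for what appears to be a timed ceremony or cinematic sequence.
; After a long delay on BeginPlay it nudges the torch mesh, reveals the actor with a walk animation, then spawns a Fire effect at a fixed location.
; Separately, Space toggles spline movement: a gated Tick feeds accumulated time to MoveMan, which positions and orients the skeletal mesh until a TotalTime timer closes the gate.
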(event Custom|BeginSpline
  (Variables|Default|SetIsMoveState true)
  (Utilities|Time|SetTimerbyEvent (delegate Custom|EndSpline) (Variables|Default|GetTotalTime))
  (Utilities|FlowControl|Gate true) ; enters at Open
)

(event Custom|EndSpline
  (Variables|Default|SetIsMoveState false)
  (Utilities|FlowControl|Gate true) ; enters at Close
)

(event EventBeginPlay
  (bind _mesh_torch (Variables|Default|GetMesh_Torch))
  (bind _relativelocation (Variables|/Script/Engine.SceneComponent|GetRelativeLocation _mesh_torch))
  (Input|EnableInput (Game|GetPlayerController 0))
  (Utilities|FlowControl|Delay 48.0)
  (Utilities|FlowControl|Sequence
    (:then_0
      (Transformation|SetRelativeLocation _mesh_torch (Math|Vector|MakeVector (.x _relativelocation) (+ (.y _relativelocation) (* (Variables|Default|GetVelocity) 2.0)) (.z _relativelocation)) false false))
    (:then_1
      (Components|Animation|PlayAnimation (Variables|Default|GetSkeletalMesh) "/Game/Model/Model/FreeWalk/Standing_Torch_Walk_Forward_Anim_mixamo_com.Standing_Torch_Walk_Forward_Anim_mixamo_com" false)
      (Rendering|SetActorHiddenInGame false)
      (Utilities|FlowControl|Delay 3.0)
      (Niagara|SpawnSystematLocation (Variables|Default|GetFire) "0.000000,-5000.000000,4000.000000"))))

(event Collision|EventActorBeginOverlap
  (params (OtherActor :type Actor%20Object%20Reference)))

(event EventTick
  (params (DeltaSeconds :type Float%20%28single-precision%29))
  (Variables|Default|SetDeltaTime DeltaSeconds)
  (Utilities|FlowControl|Gate true
    (:Exit
      (Variables|Default|SetCurTime (+ (Variables|Default|GetCurTime) (Variables|Default|GetDeltaTime)))
      (CallFunction|MoveMan (Variables|Default|GetCurTime) (Variables|Default|GetTotalTime)))))

(event Input|KeyboardEvents|SpaceBar
  (params (Key :type Key%20Structure :default "None"))
  (:Pressed
    (if (Variables|Default|GetIsMoveState)
      (CallFunction|EndSpline)
      (else
        (CallFunction|BeginSpline)))))

(fn ConstructionScript)

(fn MoveMan
  (params (CurTime :type Float%20%28single-precision%29) (TotalTime :type Float%20%28single-precision%29))
  (bind _spline (Variables|Default|GetSpline))
  (bind _returnvalue (Spline|GetSplineLength _spline))
  (bind _returnvalue_2 (/ (Variables|Default|GetCurTime) (Variables|Default|GetTotalTime)))
  (bind _returnvalue_3 (* _returnvalue_2 _returnvalue))
  (LocalVariables|SetCurTimeTemp CurTime)
  (LocalVariables|SetTotalTimeTemp TotalTime)
  (Transformation|SetRelativeTransform (Variables|Default|GetSkeletalMesh) (Math|Transform|MakeTransform (Spline|GetLocationatDistanceAlongSpline _spline _returnvalue_3 "Local") (Math|Rotator|MakeRotationfromAxes (Spline|GetDirectionatDistanceAlongSpline _spline _returnvalue_3 "Local") "0, 0, 0" "0, 0, 0") "1,1,1") false false))