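; Audio manager that sequences the soundtrack of a staged ceremony with lights-out cheers, crowd formations, fireworks, Olympic-ring and petal particles, torch and finale.
; Four entry events start the cheer, crowd stage one, fireworks and torch segments.
; Hard-coded Delays chain clips within segments, with fireworks continuing through particles into crowd stage two and torch into the ending.
; A short noise clip fills some gaps between or after clips.
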(event Custom|CheerAudioPlay
  ;[1 1 1] 灭灯欢呼
  (Audio|Components|Audio|Play (Variables|Default|GetCheer_Audio) 0.0))

(event Custom|CrowdStage1Audio1Play
  ;[1 1 1] 方阵一阶段
  (Audio|Components|Audio|Play (Variables|Default|GetCrowdStage1_Audio1) 0.0)
  (Utilities|FlowControl|Delay 28.0)
  (CallFunction|CrowdStage1Audio2Play))

(event Custom|CrowdStage2Audio2Play
  ;[1 1 1] 粒子效果阶段（五环+花瓣）
  (Audio|Components|Audio|Play (Variables|Default|GetCrowdStage2_Audio2) 0.0)
  (Utilities|FlowControl|Delay 24.0)
  (CallFunction|CrowdStage2Audio3Play))

(event Custom|CrowdStage2Audio3Play
  ;[1 1 1] 粒子效果阶段（五环+花瓣）
  (Audio|Components|Audio|Play (Variables|Default|GetCrowdStage2_Audio3) 14.0)
  (Utilities|FlowControl|Delay 55.0)
  (Audio|Components|Audio|Play (Variables|Default|GetNoiseForFill2Sec_Audio) 0.0))

(event Custom|FireTorchAudioPlay
  ;[1 1 1] 火炬+终场
  (Audio|Components|Audio|Play (Variables|Default|GetFireTorch_Audio) 0.0)
  (Utilities|FlowControl|Delay 1.2e+02)
  (CallFunction|EndingAudioPlay))

(event Custom|EndingAudioPlay
  ;[1 1 1] 火炬+终场
  (Audio|Components|Audio|Play (Variables|Default|GetEnding_Audio) 0.0))

(event Custom|CrowdStage1Audio2Play
  ;[1 1 1] 方阵一阶段
  (Audio|Components|Audio|Play (Variables|Default|GetCrowdStage1_Audio2) 0.0)
  (Utilities|FlowControl|Delay 19.0)
  (CallFunction|CrowdStage1Audio3Play))

(event Custom|CrowdStage1Audio3Play
  ;[1 1 1] 方阵一阶段
  (Audio|Components|Audio|Play (Variables|Default|GetCrowdStage1_Audio3) 0.0)
  (Utilities|FlowControl|Delay 1e+01)
  (Audio|Components|Audio|Play (Variables|Default|GetNoiseForFill2Sec_Audio) 0.0)
  (Utilities|FlowControl|Delay 2.0)
  (Audio|Components|Audio|Play (Variables|Default|GetNoiseForFill2Sec_Audio) 0.0)
  (Utilities|FlowControl|Delay 2.0)
  (CallFunction|CrowdStage1Audio4Play))

(event Custom|CrowdStage1Audio4Play
  ;[1 1 1] 方阵一阶段
  (Audio|Components|Audio|Play (Variables|Default|GetCrowdStage1_Audio4) 0.0))

(event Custom|FireworkAudioPlay
  ;[1 1 1] 焰火一阶段
  (Audio|Components|Audio|Play (Variables|Default|GetFireworkStage1_Audio) 0.0)
  (Utilities|FlowControl|Delay 31.0)
  (Audio|Components|Audio|Play (Variables|Default|GetNoiseForFill2Sec_Audio) 0.0)
  (Utilities|FlowControl|Delay 0.2)
  (CallFunction|ParticleAudio1Play))

(event Custom|ParticleAudio2Play
  ;[1 1 1] 粒子效果阶段（五环+花瓣）
  (Audio|Components|Audio|Play (Variables|Default|GetParticle_Audio2) 0.0)
  (Utilities|FlowControl|Delay 67.0)
  (CallFunction|CrowdStage2Audio1Play))

(event Custom|ParticleAudio1Play
  ;[1 1 1] 粒子效果阶段（五环+花瓣）
  (Audio|Components|Audio|Play (Variables|Default|GetParticle_Audio1) 0.0)
  (Utilities|FlowControl|Delay 36.0)
  (CallFunction|ParticleAudio2Play))

(event Custom|CrowdStage2Audio1Play
  ;[1 1 1] 粒子效果阶段（五环+花瓣）
  (Audio|Components|Audio|Play (Variables|Default|GetCrowdStage2_Audio1) 0.0)
  (Utilities|FlowControl|Delay 4e+01)
  (CallFunction|CrowdStage2Audio2Play))

(fn ConstructionScript)