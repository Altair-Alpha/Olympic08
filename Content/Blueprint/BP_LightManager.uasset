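; BP_LightManager is a level light manager that dims the scene's top spot, point and rect lights through a LightOff event.
; On BeginPlay it gathers actors tagged TopSpotLight, TopPointLight and TopRectLight, casts them and stores them in three arrays.
; LightOff plays the TurnOffLight timeline, whose separate curve for each light type sets the intensity of every cached light on each update.
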(event Custom|LightOff
  (bind (_direction _spotlightintensity _pointlightintensity _rectlightintensity) (Timeline|TurnOffLight Play)
    (:Update
      (Utilities|FlowControl|Sequence
        (:then_0
          (for _array_element (Variables|Default|GetTopSpotLights)
            (Rendering|Components|Light|SetIntensity (Variables|/Script/Engine.SpotLight|GetSpotLightComponent _array_element) _spotlightintensity)))
        (:then_1
          (for _array_element_2 (Variables|Default|GetTopPointLights)
            (Rendering|Components|Light|SetIntensity (Variables|/Script/Engine.PointLight|GetPointLightComponent _array_element_2) _pointlightintensity)))
        (:then_2
          (for _array_element_3 (Variables|Default|GetTopRectLights)
            (Rendering|Components|Light|SetIntensity (Variables|/Script/Engine.RectLight|GetRectLightComponent _array_element_3) _rectlightintensity)))))))

(event EventBeginPlay
  ;[1 1 1] 将场景中的灯光存入数组
  (Utilities|FlowControl|Sequence
    (:then_0
      (bind _outactors (Actor|GetAllActorswithTag "TopSpotLight"))
      (for _array_element _outactors
        (bind _asspot_light (Utilities|Casting|CastToSpotLight _array_element))
        (Utilities|Array|Add (Variables|Default|GetTopSpotLights) _asspot_light)))
    (:then_1
      (bind _outactors_2 (Actor|GetAllActorswithTag "TopPointLight"))
      (for _array_element_2 _outactors_2
        (bind _aspoint_light (Utilities|Casting|CastToPointLight _array_element_2))
        (Utilities|Array|Add (Variables|Default|GetTopPointLights) _aspoint_light)))
    (:then_2
      (bind _outactors_3 (Actor|GetAllActorswithTag "TopRectLight"))
      (for _array_element_3 _outactors_3
        (bind _asrect_light (Utilities|Casting|CastToRectLight _array_element_3))
        (Utilities|Array|Add (Variables|Default|GetTopRectLights) _asrect_light)))))

(fn ConstructionScript)