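; BP_LightInside is a directional light actor that the player switches and recolors from the keyboard.
; It enables player input on BeginPlay, and its construction script applies the configured initial color and intensity.
; W toggles the light by setting its color to black for off, always returning to blue for on.
; E alternates red and blue with matching intensities, independently of the on/off flag.
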(event EventBeginPlay
  ;[1 1 1] W开关灯 E变色
  (Input|EnableInput (Game|GetPlayerController 0)))

(event Collision|EventActorBeginOverlap
  (params (OtherActor :type Actor%20Object%20Reference)))

(event EventTick
  (params (DeltaSeconds :type Float%20%28single-precision%29)))

(event Input|KeyboardEvents|W
  (params (Key :type Key%20Structure :default "None"))
  (bind _directionallight (Variables|Default|GetDirectionalLight))
  ;[1 1 1] W开关灯 E变色
  (:Pressed
    (if (Variables|Default|GetLighting)
      (Rendering|Components|Light|SetLightColor _directionallight "(R=0.000000,G=0.000000,B=0.000000,A=1.000000)" true)
      (Variables|Default|SetLighting false)
      (else
        (Rendering|Components|Light|SetLightColor _directionallight (Variables|Default|GetBlue) true)
        (Rendering|Components|Light|SetIntensity _directionallight (Variables|Default|GetBlueLightIntensity))
        (Variables|Default|SetLighting true)))))

(event Input|KeyboardEvents|E
  (params (Key :type Key%20Structure :default "None"))
  (bind _directionallight (Variables|Default|GetDirectionalLight))
  ;[1 1 1] W开关灯 E变色
  (:Pressed
    (if (Variables|Default|GetColorSituation)
      (Rendering|Components|Light|SetLightColor _directionallight (Variables|Default|GetRed) true)
      (Rendering|Components|Light|SetIntensity _directionallight (Variables|Default|GetRedLightIntensity))
      (Variables|Default|SetColorSituation false)
      (else
        (Rendering|Components|Light|SetLightColor _directionallight (Variables|Default|GetBlue) true)
        (Rendering|Components|Light|SetIntensity _directionallight (Variables|Default|GetBlueLightIntensity))
        (Variables|Default|SetColorSituation true)))))

(fn ConstructionScript
  (bind _directionallight (Variables|Default|GetDirectionalLight))
  (Rendering|Components|Light|SetLightColor _directionallight (Variables|MyProperty|GetLightColor) true)
  (Rendering|Components|Light|SetIntensity _directionallight (Variables|MyProperty|GetLightIntensity)))