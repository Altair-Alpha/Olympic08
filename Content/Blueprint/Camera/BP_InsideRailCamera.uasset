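; BP_InsideRailCamera is a rail camera that the player slides along its track with the MoveForward axis.
; Axis input scaled by Velocity is added to CurrentPositionOnRail, modulo 1.0 and without delta-time scaling.
; SetViewTarget switches player 0's view to the actor spawned by its ChildActor component.
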(event Collision|EventActorBeginOverlap
  (params (OtherActor :type Actor%20Object%20Reference)))

(event EventTick
  (params (DeltaSeconds :type Float%20%28single-precision%29)))

(event EventSetViewTarget
  (Game|Player|SetViewTargetwithBlend (Game|GetPlayerController 0) (Variables|/Script/Engine.ChildActorComponent|GetChildActor (Variables|Default|GetChildActor)) 0.0 "VTBlend_Linear" 0.0 false))

(event Input|AxisEvents|InputAxisMoveForward
  (params (AxisValue :type Float%20%28single-precision%29))
  ;[1 1 1] 滑轨相机滑动
  (Variables|Default|SetCurrentPositionOnRail (Math|Float|%(Float) (+ (* AxisValue (Variables|Default|GetVelocity)) (Variables|Default|GetCurrentPositionOnRail)) 1.0)))

(fn ConstructionScript)