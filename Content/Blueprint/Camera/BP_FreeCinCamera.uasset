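; BP_FreeCinCamera is a free-flying camera actor, named for cinematic use, moved and rotated directly by player input axes.
; MoveForward and MoveRight offset it along its local axes, while MoveUp offsets it along world Z, all scaled by Velocity without sweep.
; TurnUp and TurnRight add PerDegree-scaled input to pitch and yaw, keeping roll.
; Movement applies per input call with no delta-time scaling, and BeginPlay is empty.
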(event EventBeginPlay
  ;[1 1 1] 开始时获取控制器权限
)

(event Collision|EventActorBeginOverlap
  (params (OtherActor :type Actor%20Object%20Reference)))

(event EventTick
  (params (DeltaSeconds :type Float%20%28single-precision%29)))

(event Input|AxisEvents|InputAxisMoveForward
  (params (AxisValue :type Float%20%28single-precision%29))
  ;[1 1 1] 设置前进移动
  (Transformation|AddActorLocalOffset (Math|Vector|MakeVector (* AxisValue (Variables|Default|GetVelocity)) 0.0 0.0) false false))

(event Input|AxisEvents|InputAxisMoveRight
  (params (AxisValue :type Float%20%28single-precision%29))
  ;[1 1 1] 设置左右移动
  (Transformation|AddActorLocalOffset (Math|Vector|MakeVector 0.0 (* AxisValue (Variables|Default|GetVelocity)) 0.0) false false))

(event Input|AxisEvents|InputAxisMoveUp
  (params (AxisValue :type Float%20%28single-precision%29))
  ;[1 1 1] 控制上下移动
  (Transformation|AddActorWorldOffset (Math|Vector|MakeVector 0.0 0.0 (* AxisValue (Variables|Default|GetVelocity)))))

(event Input|AxisEvents|InputAxisTurnUp
  (params (AxisValue :type Float%20%28single-precision%29))
  (bind _returnvalue (Transformation|GetActorRotation))
  ;[1 1 1] 上下转向
  (Transformation|SetActorRotation (Math|Rotator|MakeRotator (.roll _returnvalue) (+ (* AxisValue (Variables|Default|GetPerDegree)) (.pitch _returnvalue)) (.yaw _returnvalue))))

(event Input|AxisEvents|InputAxisTurnRight
  (params (AxisValue :type Float%20%28single-precision%29))
  (bind _returnvalue (Transformation|GetActorRotation))
  ;[1 1 1] 左右转向
  (Transformation|SetActorRotation (Math|Rotator|MakeRotator (.roll _returnvalue) (.pitch _returnvalue) (+ (* AxisValue (Variables|Default|GetPerDegree)) (.yaw _returnvalue)))))

(fn ConstructionScript)