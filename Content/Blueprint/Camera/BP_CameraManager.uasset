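; BP_CameraManager switches the player's view between the cameras in its Cameras array using keyboard hotkeys.
; Its construction script builds a camera type list from each camera's first tag, which GetCurCamType reads by current camera ID.
; SwitchCamera tells the chosen camera to set the view target, then moves player input from the previous camera to the new one.
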(event EventBeginPlay
  (Input|EnableInput (Game|GetPlayerController 0)))

(event Input|KeyboardEvents|6
  (params (Key :type Key%20Structure :default "None"))
  (:Pressed
    (CallFunction|SwitchCamera)))

(event Input|KeyboardEvents|7
  (params (Key :type Key%20Structure :default "None"))
  (:Pressed
    (CallFunction|SwitchCamera 1)))

(event Input|KeyboardEvents|8
  (params (Key :type Key%20Structure :default "None"))
  (:Pressed
    (CallFunction|SwitchCamera 2)))

(event Input|KeyboardEvents|9
  (params (Key :type Key%20Structure :default "None"))
  (:Pressed
    (CallFunction|SwitchCamera 3)))

(event Input|KeyboardEvents|0
  (params (Key :type Key%20Structure :default "None"))
  (:Pressed
    (CallFunction|SwitchCamera 4)))

(event Input|KeyboardEvents|O
  (params (Key :type Key%20Structure :default "None"))
  (:Pressed
    (CallFunction|SwitchCamera 5)))

(event Input|KeyboardEvents|L
  (params (Key :type Key%20Structure :default "None"))
  (:Pressed
    (CallFunction|SwitchCamera 7)))

(event Input|KeyboardEvents|P
  (params (Key :type Key%20Structure :default "None"))
  (:Pressed
    (CallFunction|SwitchCamera 6)))

(fn ConstructionScript
  (CallFunction|InitAllCameraTypes))

(fn InitAllCameraTypes
  (for _array_element (Variables|Default|GetCameras)
    (if (> (Utilities|Array|Length (Variables|/Script/Engine.Actor|GetTags _array_element)) 0)
      (Utilities|Array|Add (Variables|Default|GetCameraTypes) (Utilities|String|ToString(Name) (Utilities|Array|Get(acopy) (Variables|/Script/Engine.Actor|GetTags _array_element)))))))

(fn GetCurCamType
  (if (Variables|Default|GetIsCameraValid)
    (return (Utilities|Array|Get(acopy) (Variables|Default|GetCameraTypes) (Variables|Default|GetCurCameraID)))))

(fn SwitchCamera
  (params (CameraID :type Integer))
  (bind _returnvalue (Game|GetPlayerController 0))
  (bind _cameras (Variables|Default|GetCameras))
  (bind _output (Utilities|Array|Get(acopy) _cameras CameraID))
  (Variables|Default|SetIsCameraValid true)
  (Variables|Default|SetCurCameraID CameraID)
  (Class|BPICameraFunction|SetViewTarget(Message) _output)
  (Utilities|IsValid (Variables|Default|GetCurCamera)
    (:Is%20Valid
      (Input|DisableInput (Variables|Default|GetCurCamera) _returnvalue))
    (:Is%20Not%20Valid
      _))
  (bind _output_get (Variables|Default|SetCurCamera _output))
  (Input|EnableInput _output_get _returnvalue))