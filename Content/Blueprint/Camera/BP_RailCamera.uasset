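; Rail camera actor that slides a child cine camera along a rail from player input while tracking a target actor.
; Construction script casts the child actor to CineCameraActor and enables its look-at tracking on LookAtTargetActor.
; BeginPlay enables input for player 0, and the MoveForward axis, scaled by Velocity, offsets CurrentPositionOnRail modulo 1, without delta-time scaling.
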(event EventBeginPlay
  (Input|EnableInput (Game|GetPlayerController 0)))

(event Collision|EventActorBeginOverlap
  (params (OtherActor :type Actor%20Object%20Reference)))

(event EventTick
  (params (DeltaSeconds :type Float%20%28single-precision%29)))

(event Input|AxisEvents|InputAxisMoveForward
  (params (AxisValue :type Float%20%28single-precision%29))
  ;[1 1 1] 滑轨相机滑动
  (Variables|Default|SetCurrentPositionOnRail (Math|Float|%(Float) (+ (* AxisValue (Variables|Default|GetVelocity)) (Variables|Default|GetCurrentPositionOnRail)) 1.0)))

(fn ConstructionScript
  (CallFunction|InitLookatTarget))

(fn InitLookatTarget
  (bind _ascine_camera_actor (Utilities|Casting|CastToCineCameraActor (Variables|/Script/Engine.ChildActorComponent|GetChildActor (Variables|Default|GetChildActor))))
  (Variables|/Script/CinematicCamera.CineCameraActor|SetLookatTrackingSettings _ascine_camera_actor (Utilities|Struct|MakeCameraLookatTrackingSettings true false 0.0 (Utilities|ResolveSoftReference (Variables|Default|GetLookAtTargetActor)))))