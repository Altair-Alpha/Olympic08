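; BP_InsideCraneCamera is a player-controllable crane camera that can become player 0's view target through its SetViewTarget event.
; The MoveForward, TurnUp and TurnRight axes accumulate into crane arm length, pitch and yaw, scaled by velocity variables and clamped to limits.
; The graph only updates these values and does not apply them to components, with Tick disabled and the construction script empty.
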(event Collision|EventActorBeginOverlap
  (params (OtherActor :type Actor%20Object%20Reference)))

(event EventTick
  (params (DeltaSeconds :type Float%20%28single-precision%29)))

(event EventSetViewTarget
  (Game|Player|SetViewTargetwithBlend (Game|GetPlayerController 0) self 0.0 "VTBlend_Linear" 0.0 false))

(event Input|AxisEvents|InputAxisMoveForward
  (params (AxisValue :type Float%20%28single-precision%29))
  ;[1 1 1] 控制Arm长度
  (Variables|Default|SetCraneArmLength (Math|Float|Clamp(Float) (+ (Variables|Default|GetCraneArmLength) (* AxisValue (Variables|Default|GetArmVelocity))) (Variables|Default|GetMInArmLen) (Variables|Default|GetMaxArmLen))))

(event Input|AxisEvents|InputAxisTurnUp
  (params (AxisValue :type Float%20%28single-precision%29))
  ;[1 1 1] 控制Pitch方向转向
  (Variables|Default|SetCranePitch (Math|Float|Clamp(Float) (+ (Variables|Default|GetCranePitch) (* AxisValue (Variables|Default|GetTurnVelocity))) 0.0 9e+01)))

(event Input|AxisEvents|InputAxisTurnRight
  (params (AxisValue :type Float%20%28single-precision%29))
  ;[1 1 1] 控制Yaw方向转向
  (Variables|Default|SetCraneYaw (Math|Float|Clamp(Float) (+ (Variables|Default|GetCraneYaw) (* AxisValue (Variables|Default|GetTurnVelocity))) -9e+01 9e+01)))

(fn ConstructionScript)