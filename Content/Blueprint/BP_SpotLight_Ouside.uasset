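; Outdoor spotlight actor that sweeps its beam automatically and can be switched on and off by the player.
; Two timelines, each started after a random delay of up to five seconds, drive hinge yaw and light container pitch, so instances can move out of sync.
; It enables player input; Q prints a debug string and flips its own Working flag, setting SpotLight intensity on every instance of the class.
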(event EventBeginPlay
  (Utilities|FlowControl|Sequence
    (:then_0
      ;[1 1 1] 聚光灯转动
      (Utilities|FlowControl|Sequence
        (:then_0
          (Utilities|FlowControl|Delay (* (Math|Random|RandomFloat) 5.0))
          (bind _newtrack_0 (Timeline|Timeline_0 Play)
            (:Update
              (Transformation|SetRelativeRotation (Variables|Default|GetHinge) (Math|Rotator|MakeRotator 0.0 0.0 _newtrack_0) false false))))
        (:then_1
          (Utilities|FlowControl|Delay (* (Math|Random|RandomFloat) 5.0))
          (bind _newtrack_0_2 (Timeline|Timeline_1 Play)
            (:Update
              (Transformation|SetRelativeRotation (Variables|Default|GetLightContainer) (Math|Rotator|MakeRotator 0.0 _newtrack_0_2 0.0) false false))))))
    (:then_1
      (Input|EnableInput (Game|GetPlayerController 0)))))

(event Collision|EventActorBeginOverlap
  (params (OtherActor :type Actor%20Object%20Reference))
  (|CallParentFunction OtherActor) ; This node is disabled and will not be called.\nDrag off pins to build functionality.
)

(event EventTick
  (params (DeltaSeconds :type Float%20%28single-precision%29))
  (|CallParentFunction DeltaSeconds) ; This node is disabled and will not be called.\nDrag off pins to build functionality.
)

(event Input|KeyboardEvents|Q
  (params (Key :type Key%20Structure :default "None"))
  (:Pressed
    (Development|PrintString "111")
    (bind _outactors (Actor|GetAllActorsOfClass "BP_SpotLight_Ouside_C"))
    (if (Variables|Default|GetWorking)
      (for _array_element _outactors
        (Rendering|Components|Light|SetIntensity (Variables|/Game/Blueprint/BP_SpotLight.BP_SpotLight_C|GetSpotLight _array_element) 0.0)
        (Variables|Default|SetWorking false))
      (else
        (for _array_element_2 _outactors
          (Rendering|Components|Light|SetIntensity (Variables|/Game/Blueprint/BP_SpotLight.BP_SpotLight_C|GetSpotLight _array_element_2) 6e+02)
          (Variables|Default|SetWorking true))))))

(fn ConstructionScript
  (|CallParentFunction))